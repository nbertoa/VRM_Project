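; Performer skeleton visualizer that shows upper-body and hip bone transforms as nine joint components linked by debug lines.
; Each Tick it fetches the performer's bone transforms and places the joints relative to the hip, at a fixed world-space X offset.
; Only the head also takes its bone's rotation.
; JointLinkIdx pairs each array index with another joint index to draw the connecting debug cylinders.
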(event `self.ReceiveBeginPlay`
  (`self.InitializeJoints`))

(event `self.ReceiveTick`
  (params (DeltaSeconds :type "Float (single-precision)"))
  (bind _transforms (`/Game/Sandbox/VMC_test/Blueprints/VMCLibrary.GetPerformartBoneTransform`))
  (`self.SetJointTransformsAndDrawLinks` _transforms))

(fn `Adjust Joint Transforms Position`
  (params (JointTransforms :type "Array of Transform Structure"))
  (for (_array_element _array_index) (`self.Joints`)
    (`SceneComponent.K2_SetWorldLocation` _array_element (+ (- (.location (`|GetArrayItem` JointTransforms _array_index)) (.location (`|GetArrayItem` JointTransforms 8))) (110.0 0.0 0.0)) false false))
  (`SceneComponent.K2_SetWorldRotation` (`self.Head`) (.rotation (`|GetArrayItem` JointTransforms)) false false))

(fn `DrawJointLinks`
  (bind _joints (`self.Joints`))
  (for (_array_element _array_index) (`self.JointLinkIdx`)
    (`KismetSystemLibrary.DrawDebugCylinder` (`SceneComponent.K2_GetComponentLocation` (`|GetArrayItem` _joints _array_element)) (`SceneComponent.K2_GetComponentLocation` (`|GetArrayItem` _joints _array_index)) 0.5 15 (make `LinearColor` 1.0 0.5))))

(fn `InitializeJoints`
  (set `self.Joints` (`|MakeArray` (`self.Head`) (`self.Neck`) (`self.RightUpperArm`) (`self.RightLowerArm`) (`self.RightHand`) (`self.LeftUpperArm`) (`self.LeftLowerArm`) (`self.LeftHand`) (`self.Hip`))))

(fn `SetJointTransformsAndDrawLinks`
  (params (Transforms :type "Array of Transform Structure"))
  (`self.Adjust Joint Transforms Position` Transforms)
  (`self.DrawJointLinks`))

(fn `UserConstructionScript`)