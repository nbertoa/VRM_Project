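; BP_BoneSpheres is an actor that visualizes an upper-body skeleton from bone transforms, under the VMC folder.
; Each tick it caches GetBoneTransform's result and moves nine joint components, from head to hip, to hip-relative positions around the actor's location.
; It then draws red debug cylinders between joints paired through the JointLinkIdx array.
; Getter functions expose raw cached locations for head, neck, hips, hands and upper arms.
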(event `self.ReceiveBeginPlay`
  (`self.InitializeJoints`))

(event `self.ReceiveTick`
  (params (DeltaSeconds :type "Float (single-precision)"))
  (bind _transforms (`/Game/Blueprints/VMC/VMCLibrary.GetBoneTransform`))
  (bind _output_get (set `self.BoneTransforms` _transforms))
  (`self.SetJointTransformsAndDrawLinks` _output_get))

(fn `AdjustJointTransformsPosition`
  (params (JointTransforms :type "Array of Transform Structure") (PositionOffset :type "Vector Structure"))
  (for (_array_element _array_index) (`self.Joints`)
    (`SceneComponent.K2_SetWorldLocation` _array_element (+ (* (- (.location (`|GetArrayItem` JointTransforms _array_index)) (.location (`|GetArrayItem` JointTransforms 8))) 1.0) PositionOffset) false false)))

(fn `Draw Joint Links`
  (bind _joints (`self.Joints`))
  (for (_array_element _array_index) (`self.JointLinkIdx`)
    (`KismetSystemLibrary.DrawDebugCylinder` (`SceneComponent.K2_GetComponentLocation` (`|GetArrayItem` _joints _array_element)) (`SceneComponent.K2_GetComponentLocation` (`|GetArrayItem` _joints _array_index)) 0.5 15 (`KismetMathLibrary.LinearColor_Red`))))

(fn `GetHeadLocation`
  (returns (Location :type "Vector Structure"))
  (bind _output_location (`KismetMathLibrary.BreakTransform` (`|GetArrayItem` (`self.BoneTransforms`) (`self.HeadIndex`))))
  (return _output_location))

(fn `GetHipsLocation`
  (returns (Location :type "Vector Structure"))
  (bind _output_location (`KismetMathLibrary.BreakTransform` (`|GetArrayItem` (`self.BoneTransforms`) (`self.HipsIndex`))))
  (return _output_location))

(fn `GetLeftHandLocation`
  (returns (Location :type "Vector Structure"))
  (bind _output_location (`KismetMathLibrary.BreakTransform` (`|GetArrayItem` (`self.BoneTransforms`) (`self.LeftHandIndex`))))
  (return _output_location))

(fn `GetLeftUpperArmLocation`
  (returns (Location :type "Vector Structure"))
  (bind _output_location (`KismetMathLibrary.BreakTransform` (`|GetArrayItem` (`self.BoneTransforms`) (`self.LeftUpperArmIndex`))))
  (return _output_location))

(fn `GetNeckLocation`
  (returns (Location :type "Vector Structure"))
  (bind _output_location (`KismetMathLibrary.BreakTransform` (`|GetArrayItem` (`self.BoneTransforms`) (`self.NeckIndex`))))
  (return _output_location))

(fn `GetRightHandLocation`
  (returns (Location :type "Vector Structure"))
  (bind _output_location (`KismetMathLibrary.BreakTransform` (`|GetArrayItem` (`self.BoneTransforms`) (`self.RightHandIndex`))))
  (return _output_location))

(fn `GetRightUpperArmLocation`
  (returns (Location :type "Vector Structure"))
  (bind _output_location (`KismetMathLibrary.BreakTransform` (`|GetArrayItem` (`self.BoneTransforms`) (`self.RightUpperArmIndex`))))
  (return _output_location))

(fn `InitializeJoints`
  (set `self.Joints` (`|MakeArray` (`self.Head`) (`self.Neck`) (`self.RightUpperArm`) (`self.RightLowerArm`) (`self.RightHand`) (`self.LeftUpperArm`) (`self.LeftLowerArm`) (`self.LeftHand`) (`self.Hip`))))

(fn `SetJointTransformsAndDrawLinks`
  (params (Transforms :type "Array of Transform Structure"))
  (`self.AdjustJointTransformsPosition` Transforms (`self.K2_GetActorLocation`))
  (`self.Draw Joint Links`))

(fn `UserConstructionScript`)